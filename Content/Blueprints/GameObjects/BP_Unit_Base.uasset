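; BP_Unit_Base is a base Blueprint for game units that sets up modular hardpoints held in child actor components.
; On BeginPlay it initializes the engine hardpoint, then the shield generator hardpoint, casting each child actor to its Blueprint class and making the unit its owner.
; The engine then attaches its movement component and the shield generator initializes its shield settings, so both behaviors are delegated to the hardpoint actors.
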(event `self.ReceiveBeginPlay`
  (`self.InitializeEngine`)
  (`self.InitializeShieldGenerator`))

(fn `InitializeEngine`
  (bind _asbp_hardpoint_engine (cast `/Game/Blueprints/GameObjects/BP_Hardpoint_Engine` (`ChildActorComponent.ChildActor` (`self.HardpointEngine`))))
  (`self.SetOwner` _asbp_hardpoint_engine self)
  (`HardpointEngine.AttachMovementComponent` _asbp_hardpoint_engine))

(fn `InitializeShieldGenerator`
  (bind _asbp_hardpoint_shield_generator (cast `/Game/Blueprints/GameObjects/BP_Hardpoint_ShieldGenerator` (`ChildActorComponent.ChildActor` (`self.HardpointShieldGenerator`))))
  (`self.SetOwner` _asbp_hardpoint_shield_generator self)
  (`HardpointShieldGenerator.InitializeShieldSettings` _asbp_hardpoint_shield_generator))

(fn `UserConstructionScript`)